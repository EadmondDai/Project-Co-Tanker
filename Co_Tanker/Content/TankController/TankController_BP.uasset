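; Player controller for a tank with separate driver and gunner roles, chosen by an IsGunner flag.
; Look input rotates the body's camera gimbals for the driver, or the turret and zenith gimbal for the gunner.
; Track throttles drive the body's two tracks, a test axis nudges the pawn forward, and Fire triggers on the controlled Tank.
; CreateUI adds a gunner widget for gunners, though nothing here calls it.
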(event EventBeginPlay)

(event EventTick
  (params (DeltaSeconds :type Float%20%28single-precision%29)))

(event Input|ActionEvents|InputActionFire
  (params (Key :type Key%20Structure :default "AnyKey"))
  (:Released
    (bind _astank (Utilities|Casting|CastToTank (Pawn|GetControlledPawn)))
    (Class|Tank|Fire _astank)))

(event Input|AxisEvents|InputAxisLookHorizontal
  (params (AxisValue :type Float%20%28single-precision%29))
  (if (!= AxisValue 0.0)
    (if (Variables|Default|GetbIsGunner)
      (CallFunction|GunLookHorizontal AxisValue)
      (else
        (CallFunction|BodyLookHorizontal AxisValue)))))

(event Input|AxisEvents|InputAxisLookVertical
  (params (AxisValue :type Float%20%28single-precision%29))
  (if (!= AxisValue 0.0)
    (if (Variables|Default|GetbIsGunner)
      (CallFunction|GunLookVertical AxisValue)
      (else
        (CallFunction|BodyLookVertical AxisValue)))))

(event Input|AxisEvents|InputAxisRightTrackThrottle
  (params (AxisValue :type Float%20%28single-precision%29))
  (bind _astank_body_bp (Utilities|Casting|CastToTankBody_BP (Pawn|GetControlledPawn)))
  (Class|TankTrack|SetThrottle (Variables|/Game/Tank/TankBody_BP.TankBody_BP_C|GetRightTrack _astank_body_bp) AxisValue))

(event Input|AxisEvents|InputAxisMoveForwardTest
  (params (AxisValue :type Float%20%28single-precision%29))
  (bind _returnvalue (Pawn|GetControlledPawn))
  (if (!= AxisValue 0.0)
    (if (not (Variables|Default|GetbIsGunner))
      (Transformation|AddLocalOffset (VehicleSound|GetRootComponent _returnvalue) (* (Transformation|GetActorForwardVector _returnvalue) AxisValue) false false))))

(event Input|AxisEvents|InputAxisLeftTrackThrottle
  (params (AxisValue :type Float%20%28single-precision%29))
  (bind _astank_body_bp (Utilities|Casting|CastToTankBody_BP (Pawn|GetControlledPawn)))
  (Class|TankTrack|SetThrottle (Variables|/Game/Tank/TankBody_BP.TankBody_BP_C|GetLeftTrack _astank_body_bp) AxisValue))

(fn ConstructionScript)

(fn BodyLookHorizontal
  (params (delta :type Float%20%28single-precision%29))
  (bind _astank_body_bp (Utilities|Casting|CastToTankBody_BP (Pawn|GetControlledPawn)))
  (Transformation|AddLocalRotation (Variables|/Game/Tank/TankBody_BP.TankBody_BP_C|GetAzimuthGimbal _astank_body_bp) (Math|Rotator|MakeRotator 0.0 0.0 (* delta (Utilities|Time|GetWorldDeltaSeconds) 1e+02)) false false))

(fn BodyLookVertical
  (params (delta :type Float%20%28single-precision%29))
  (bind _astank_body_bp (Utilities|Casting|CastToTankBody_BP (Pawn|GetControlledPawn)))
  (Transformation|AddLocalRotation (Variables|/Game/Tank/TankBody_BP.TankBody_BP_C|GetSpringArm _astank_body_bp) (Math|Rotator|MakeRotator 0.0 (* delta (Utilities|Time|GetWorldDeltaSeconds) 1e+02) 0.0) false false))

(fn GunLookHorizontal
  (params (delta :type Float%20%28single-precision%29))
  (bind _astank_turret_bp (Utilities|Casting|CastToTankTurret_BP (Pawn|GetControlledPawn)))
  (Class|Turret|Rotate (Variables|/Game/Tank/TankTurret_BP.TankTurret_BP_C|GetTurret _astank_turret_bp) delta))

(fn GunLookVertical
  (params (delta :type Float%20%28single-precision%29))
  (bind _astank_turret_bp (Utilities|Casting|CastToTankTurret_BP (Pawn|GetControlledPawn)))
  (Transformation|AddLocalRotation (Variables|/Game/Tank/TankTurret_BP.TankTurret_BP_C|GetZenithGimbal _astank_turret_bp) (Math|Rotator|MakeRotator 0.0 (* delta (Utilities|Time|GetWorldDeltaSeconds) 1e+01) 0.0) false false))

(fn CreateUI
  (if (Variables|Default|GetbIsGunner)
    (bind _returnvalue (UserInterface|CreateWidget "/Game/UI/GunnerUI_BP.GunnerUI_BP_C" self))
    (UserInterface|Viewport|AddtoPlayerScreen _returnvalue)
    (Variables|Default|SetGunnerUI _returnvalue)))