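; Game mode for local co-op tank play, where one player drives the tank body and a second player gunner controls its turret.
; On BeginPlay it spawns and possesses a tank body at the first PlayerStart, creates a second local player flagged as gunner, and creates that player's UI.
; CreateTankPlayerPawn spawns either a turret snapped to the driver's TurretNeck socket or a separate body, using the second PlayerStart.
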(event Custom|CreateTankPlayerPawn
  (params (TankController :type Tank%20Controller%20BP%20Object%20Reference) (IsGunner :type Boolean))
  (bind _returnvalue (Pawn|GetControlledPawn TankController))
  (bind _spawnpoints (Variables|Default|GetSpawnPoints))
  (bind _output (Utilities|Array|Get(acopy) _spawnpoints 1))
  (bind _returnvalue_2 (Transformation|GetActorTransform _output))
  (bind _output_get (Variables|/Script/Co_Tanker.TankController|SetbIsGunner TankController IsGunner))
  (Utilities|IsValid _returnvalue
    (:Is%20Valid
      (Actor|DestroyActor _returnvalue))
    (:Is%20Not%20Valid
      _))
  (if _output_get
    (bind _returnvalue_3 (Game|SpawnActorfromClass "/Game/Tank/TankTurret_BP.TankTurret_BP_C" _returnvalue_2 "Undefined" 0 0))
    (Pawn|Possess TankController _returnvalue_3)
    (Game|Player|SetViewTargetwithBlend TankController _returnvalue_3 0.0 "VTBlend_Linear" 0.0 false)
    (bind _astank_body_bp (Utilities|Casting|CastToTankBody_BP (Pawn|GetControlledPawn (Game|GetPlayerController 0))))
    (Transformation|AttachComponentToComponent _returnvalue_3 (Variables|/Game/Tank/TankBody_BP.TankBody_BP_C|GetTurretNeck _astank_body_bp) "Turret" "SnapToTarget" "SnapToTarget" "SnapToTarget" true)
    (else
      (bind _returnvalue_4 (Game|SpawnActorfromClass "/Game/Tank/TankBody_BP.TankBody_BP_C" _returnvalue_2 "Undefined" 0 0))
      (Pawn|Possess TankController _returnvalue_4)
      (Game|Player|SetViewTargetwithBlend TankController _returnvalue_4 0.0 "VTBlend_Linear" 0.0 false))))

(event EventTick
  (params (DeltaSeconds :type Float%20%28single-precision%29)))

(event EventBeginPlay
  (bind _returnvalue (Game|GetPlayerController 0))
  (bind _outactors (Actor|GetAllActorsOfClass "/Script/Engine.PlayerStart"))
  (Variables|Default|SetSpawnPoints _outactors)
  (bind _returnvalue_2 (Game|SpawnActorfromClass "/Game/Tank/TankBody_BP.TankBody_BP_C" (Transformation|GetActorTransform (Utilities|Array|Get(acopy) (Variables|Default|GetSpawnPoints))) "Undefined" 0 0))
  (Pawn|Possess _returnvalue _returnvalue_2)
  (Game|Player|SetViewTargetwithBlend _returnvalue _returnvalue_2 0.0 "VTBlend_Linear" 0.0 false)
  (bind _returnvalue_3 (Class|GameplayStatics|CreatePlayer -1))
  (bind _astank_controller_bp (Utilities|Casting|CastToTankController_BP _returnvalue_3))
  (bind _output_get (Variables|/Script/Co_Tanker.TankController|SetbIsGunner _astank_controller_bp true))
  (CallFunction|CreateTankPlayerPawn _astank_controller_bp _output_get)
  (Default|CreateUI _astank_controller_bp))

(fn ConstructionScript)